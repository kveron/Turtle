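; BP_Button is a button actor that spawns an AI-controlled turtle when pressed.
; ButtonPressed plays a timeline that moves the Sphere on Z, with a DoOnce blocking repeat presses until it finishes.
; On finish it spawns a Turtle_Pawn just above TurtleSpawner with TurtleTarget's location as its target.
; It then spawns a Turtle_AI_BP controller carrying TurtleType, has it possess the pawn, and resets the DoOnce.
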(event `Button Pressed`
  (bind (_returnvalue_x _returnvalue_y _returnvalue_z) (`KismetMathLibrary.BreakVector` (`self.K2_GetActorLocation` (`self.TurtleSpawner`))))
  ;[1 1 1] Button pressed anim
  (`/Engine/EditorBlueprintResources/StandardMacros.DoOnce` false :!label _label
    (:`Completed`
      (bind (_direction _position) (`Timeline|ButtonPressedAnim` :!via `PlayFromStart`)
        (:`Update`
          (`SceneComponent.K2_SetRelativeLocation` (`self.Sphere`) (`KismetMathLibrary.MakeVector` 0.0 0.0 _position) false false))
        (:`Finished`
          ;[1 1 1] Spawn turtle and controller
          (bind _returnvalue (`|SpawnActorFromClass` "/Game/Blueprints/Turtle/Turtle_Pawn.Turtle_Pawn_C" (`KismetMathLibrary.MakeTransform` (`KismetMathLibrary.MakeVector` _returnvalue_x _returnvalue_y (+ _returnvalue_z 10.0))) "Undefined" "OverrideRootScale" null (`self.K2_GetActorLocation` (`self.TurtleTarget`)) null))
          (bind _returnvalue_2 (`|SpawnActorFromClass` "/Game/Blueprints/Turtle/Turtle_AI_BP.Turtle_AI_BP_C" (`self.GetTransform` _returnvalue) "Undefined" "OverrideRootScale" null (`self.TurtleType`) null))
          (`Controller.Possess` _returnvalue_2 _returnvalue)
          (goto _label :!via `Reset`))))))

(fn `UserConstructionScript`)